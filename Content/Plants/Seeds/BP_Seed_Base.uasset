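; Base actor for a pickable seed item that the player collects by walking into it.
; On begin play it applies its configured seed mesh to the Seed component.
; When the player pawn overlaps the Box, it calls AddCropsMessage on the player character with its plant type and picked amount, then destroys itself.
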(event `self.ReceiveBeginPlay`
  (`StaticMeshComponent.SetStaticMesh` (`self.Seed`) (`self.SeedMesh`)))

(event `self.Box.OnComponentBeginOverlap`
  (params (OverlappedComponent :type "PrimitiveComponent Object Reference") (OtherActor :type "Actor Object Reference") (OtherComp :type "PrimitiveComponent Object Reference") (OtherBodyIndex :type Integer) (bFromSweep :type Boolean) (SweepResult :type "HitResult Structure (by ref)"))
  (if (== OtherActor (`GameplayStatics.GetPlayerPawn` 0))
    (message `/Game/_Player/MainPlayerCharacterInterface.Add_Crops` (`GameplayStatics.GetPlayerCharacter` 0) (`self.PlantType`) (`self.AmountPicked`))
    (`self.K2_DestroyActor`)))

(fn `UserConstructionScript`)