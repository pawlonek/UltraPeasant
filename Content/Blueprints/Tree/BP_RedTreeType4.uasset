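; BP_RedTreeType4 is a damageable tree actor that counts toward an objective when destroyed.
; AnyDamage subtracts from its Health; at zero or below it prints a debug string and casts player 0's character to BP_ThirdPersonCharacter.
; It then calls that character's objective event with its ObjectiveID and a value of 1, and destroys itself.
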(event `self.ReceiveAnyDamage`
  (params (Damage :type "Float (single-precision)") (DamageType :type "DamageType Object Reference") (InstigatedBy :type "Controller Object Reference") (DamageCauser :type "Actor Object Reference"))
  (bind _output_get (set `self.Health` (- (`self.Health`) Damage)))
  (if (<= _output_get 0.0)
    (`KismetSystemLibrary.PrintString` "hit hit hit")
    (bind _asbp_third_person_character (cast `/Game/Blueprints/BP_ThirdPersonCharacter` (`GameplayStatics.GetPlayerCharacter` 0)))
    (`/Game/Blueprints/BP_ThirdPersonCharacter.OnObjectiveIDCalled` _asbp_third_person_character (`self.ObjectiveID`) 1)
    (`self.K2_DestroyActor`)))

(fn `UserConstructionScript`)