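; Farm tile actor where the player plants wheat, corn or pumpkin seeds, adds water and fertilizer, and harvests crops.
; Plant events swap three mesh stages via the GrowTime macro, a Text3D countdown shortened by hydration and fertilizer.
; Looping timers drain both resources, faster during growth, while player inventory is read and deducted through message calls.
; Activate calls Harvest, which spawns a loose crop actor and frees the tile after a short delay.
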(event `self.ReceiveBeginPlay`
  (`Text3DComponent.SetText` (`self.Text3D`) (`self.Value`))
  (set `self.FertilizerDrawSpeed` 0.01)
  (set `self.WaterDrawSpeed` 0.01))

(event `RemoveWater`
  ;[0.07812 0.07812 0.07812 1 80] Removing Water And Ferilizer Every Second
  (if (<= (`self.WaterAmount`) 0.0)
    (set `self.Hydrated` false)
    (else
      (bind _output_get (set `self.WaterAmount` (- (`self.WaterAmount`) (`self.WaterDrawSpeed`)))))))

(event `Fertilize`
  ;[0.07812 0.07812 0.07812 1 80] Removing Water And Ferilizer Every Second
  (if (<= (`self.FertilizerAmount`) 0.0)
    (set `self.Fertilized` false)
    (else
      (bind _output_get (set `self.FertilizerAmount` (- (`self.FertilizerAmount`) (`self.FertilizerDrawSpeed`)))))))

(event `StartUsingFertilizer`
  ;[0.07812 0.07812 0.07812 1 80] Removing Water And Ferilizer Every Second
  (bind _returnvalue (`KismetSystemLibrary.K2_SetTimerDelegate` (delegate `Fertilize`) 1.0 true))
  (set `self.FertilizerTimer` _returnvalue))

(event `StartDrawingWater`
  ;[0.07812 0.07812 0.07812 1 80] Removing Water And Ferilizer Every Second
  (bind _returnvalue (`KismetSystemLibrary.K2_SetTimerDelegate` (delegate `RemoveWater`) 1.0 true))
  (set `self.WaterTimer` _returnvalue))

(event `PlantWheat`
  (bind _relativetransformlocation (`self.RelativeTransformLocation`))
  ;[0.151 0.151 0.151 1 80] Growing crops
  (bind _returnvalue (`AddComponent|NODE_AddStaticMeshComponent-0` :`RelativeTransform` (`KismetMathLibrary.MakeTransform` _relativetransformlocation)))
  (`self.GrowTime` (`self.WheatGrowTIme`)
    (:`Out`
      (`ActorComponent.K2_DestroyComponent` _returnvalue)
      (bind _returnvalue_2 (`AddComponent|NODE_AddStaticMeshComponent-1` :`RelativeTransform` (`KismetMathLibrary.MakeTransform` _relativetransformlocation)))
      (`self.GrowTime` (`self.WheatGrowTIme`)
        (:`Out`
          (`ActorComponent.K2_DestroyComponent` _returnvalue_2)
          (bind _returnvalue_3 (`AddComponent|NODE_AddStaticMeshComponent-2` :`RelativeTransform` (`KismetMathLibrary.MakeTransform` _relativetransformlocation)))
          (set `self.FullyGrown?` true)
          (set `self.CurrentMesh` _returnvalue_3)
          (set `self.WhatCanBeHarvested?` "Wheat"))))))

(event `Plant Corn`
  (bind _relativetransformlocation (`self.RelativeTransformLocation`))
  ;[0.151 0.151 0.151 1 80] Growing crops
  (bind _returnvalue (`AddComponent|NODE_AddStaticMeshComponent-3` :`RelativeTransform` (`KismetMathLibrary.MakeTransform` _relativetransformlocation)))
  (`self.GrowTime` (`self.CornGrowTime`)
    (:`Out`
      (`ActorComponent.K2_DestroyComponent` _returnvalue)
      (bind _returnvalue_2 (`AddComponent|NODE_AddStaticMeshComponent-4` :`RelativeTransform` (`KismetMathLibrary.MakeTransform` _relativetransformlocation)))
      (`self.GrowTime` (`self.CornGrowTime`)
        (:`Out`
          (`ActorComponent.K2_DestroyComponent` _returnvalue_2)
          (bind _returnvalue_3 (`AddComponent|NODE_AddStaticMeshComponent-5` :`RelativeTransform` (`KismetMathLibrary.MakeTransform` _relativetransformlocation)))
          (set `self.FullyGrown?` true)
          (set `self.CurrentMesh` _returnvalue_3)
          (set `self.WhatCanBeHarvested?` "Corn"))))))

(event `PlantPumpkin`
  (bind _relativetransformlocation (`self.RelativeTransformLocation`))
  ;[0.151 0.151 0.151 1 80] Growing crops
  (bind _returnvalue (`AddComponent|NODE_AddStaticMeshComponent-6` :`RelativeTransform` (`KismetMathLibrary.MakeTransform` _relativetransformlocation)))
  (`self.GrowTime` (`self.PumpkinhGrowTime`)
    (:`Out`
      (`ActorComponent.K2_DestroyComponent` _returnvalue)
      (bind _returnvalue_2 (`AddComponent|NODE_AddStaticMeshComponent-7` :`RelativeTransform` (`KismetMathLibrary.MakeTransform` _relativetransformlocation)))
      (`self.GrowTime` (`self.PumpkinhGrowTime`)
        (:`Out`
          (`ActorComponent.K2_DestroyComponent` _returnvalue_2)
          (bind _returnvalue_3 (`AddComponent|NODE_AddStaticMeshComponent-8` :`RelativeTransform` (`KismetMathLibrary.MakeTransform` _relativetransformlocation)))
          (set `self.FullyGrown?` true)
          (set `self.CurrentMesh` _returnvalue_3)
          (set `self.WhatCanBeHarvested?` "Pumpkin"))))))

(event `/Game/Blueprints/BPI_PlantSeed_FarmTile.PlantSeed`
  (params (CropType :type "/Game/Plants/Structures/PlantsEnum Enum" :default "NewEnumerator0"))
  ;[0.05729 0.05729 0.05729 1 80] Planting Seeds By Player
  (if (not (`self.IsSomethingPlanted?`))
    (bind _seed_type (message `/Game/Blueprints/MainPlayerCharacterInterface.Get_Selected_Seed_Type` (`GameplayStatics.GetPlayerCharacter` 0)))
    (bind _we_do_have_that_seed (`self.DoWeHaveThatSeed` _seed_type))
    (if _we_do_have_that_seed
      (message `/Game/Blueprints/MainPlayerCharacterInterface.Remove_Crops_Amount` (`GameplayStatics.GetPlayerCharacter` 0) _seed_type 1)
      (switch `/Game/Plants/Structures/PlantsEnum` _seed_type
        (:`NewEnumerator1`
          (`self.PlantWheat`))
        (:`NewEnumerator3`
          (`self.Plant Corn`))
        (:`NewEnumerator5`
          (`self.PlantPumpkin`)))
      (set `self.IsSomethingPlanted?` true))))

(event `/Game/Blueprints/BPI_PlantSeed_FarmTile.HydrateField`
  (bind _returnvalue (`GameplayStatics.GetPlayerCharacter` 0))
  (bind _wateramount (`self.WaterAmount`))
  (bind _returnvalue_2 (- 5.0 _wateramount))
  ;[0.04167 0.04167 0.04167 1 80] Adding Water By Player
  (bind _newparam (message `/Game/Blueprints/MainPlayerCharacterInterface.Check_Water_Amount` _returnvalue))
  (if (>= _newparam _returnvalue_2)
    (message `/Game/Blueprints/MainPlayerCharacterInterface.Remove_Water_Amount` _returnvalue _returnvalue_2)
    (set `self.WaterAmount` 5.0)
    (set `self.Hydrated` true)
    (`self.StartDrawingWater`)
    (else
      (set `self.WaterAmount` (+ _newparam _wateramount))
      (message `/Game/Blueprints/MainPlayerCharacterInterface.Remove_Water_Amount` _returnvalue _newparam)
      (set `self.Hydrated` true)
      (`self.StartDrawingWater`))))

(event `/Game/Blueprints/BPI_PlantSeed_FarmTile.FertilizeField`
  (bind _returnvalue (`GameplayStatics.GetPlayerCharacter` 0))
  (bind _fertilizeramount (`self.FertilizerAmount`))
  (bind _returnvalue_2 (- 10.0 _fertilizeramount))
  ;[0.0625 0.0625 0.0625 1 80] Adding Fertilizer By Player
  (bind _amount (message `/Game/Blueprints/MainPlayerCharacterInterface.Check_Fertilizer_Amount` _returnvalue))
  (if (>= _amount _returnvalue_2)
    (message `/Game/Blueprints/MainPlayerCharacterInterface.Remove_Fertilizer_Amount` _returnvalue (`KismetMathLibrary.FTrunc` _returnvalue_2))
    (set `self.FertilizerAmount` 10.0)
    (set `self.Fertilized` true)
    (`self.StartUsingFertilizer`)
    (else
      (set `self.FertilizerAmount` (+ _amount _fertilizeramount))
      (message `/Game/Blueprints/MainPlayerCharacterInterface.Remove_Fertilizer_Amount` _returnvalue _amount)
      (set `self.Fertilized` true)
      (`self.StartUsingFertilizer`))))

(event `Harvest`
  (bind _returnvalue (`KismetMathLibrary.Conv_VectorToTransform` (`SceneComponent.K2_GetComponentLocation` (`self.Text3D`))))
  ;[0.04167 0.04167 0.04167 1 80] Collecting Crops
  (if (`self.FullyGrown?`)
    (`ActorComponent.K2_DestroyComponent` (`self.CurrentMesh`))
    (switch `string` (`self.WhatCanBeHarvested?`)
      (:`Default`
        _)
      (:`Wheat`
        (`|SpawnActorFromClass` "/Game/Plants/Loose/BP_Loose_Wheat.BP_Loose_Wheat_C" _returnvalue "Undefined" "OverrideRootScale" null "wheatloose" null))
      (:`Corn`
        (`|SpawnActorFromClass` "/Game/Plants/Loose/BP_Loose_Corn.BP_Loose_Corn_C" _returnvalue "Undefined" "OverrideRootScale" null "cornloose" null))
      (:`Pumpkin`
        (`|SpawnActorFromClass` "/Game/Plants/Loose/BP_Loose_Pumpkin.BP_Loose_Pumpkin_C" _returnvalue "Undefined" "OverrideRootScale" null "pumpkinloose" null)))
    (set `self.FullyGrown?` false)
    (set `self.CurrentMesh` null)
    (set `self.WhatCanBeHarvested?` "")
    (`KismetSystemLibrary.Delay` 0.2)
    (set `self.IsSomethingPlanted?` false)))

(event `/Game/Blueprints/BPI_Activate.Activate`
  ;[0.04167 0.04167 0.04167 1 80] Collecting Crops
  (`self.Harvest`))

(fn `DoWeHaveThatSeed`
  (params (Plant :type "/Game/Plants/Structures/PlantsEnum Enum" :default "NewEnumerator0"))
  (returns (`We do have that seed` :type Boolean))
  (bind _amount (message `/Game/Blueprints/MainPlayerCharacterInterface.Check_Crops_Amount` (`GameplayStatics.GetPlayerPawn` 0) Plant))
  (return (>= _amount 1)))

(fn `GetFieldParameters`
  (returns (Water :type "Float (double-precision)") (Fertilizer :type "Float (double-precision)") (Sickness :type "Float (double-precision)") (Name :type Text))
  (return (`self.WaterAmount`) (`self.FertilizerAmount`) (`self.Disease`) (`KismetTextLibrary.Conv_StringToText` (`KismetSystemLibrary.GetDisplayName` self))))

(fn `Harvest_DeprecatedBecauseOfBugs`
  (bind _returnvalue (`KismetMathLibrary.Conv_VectorToTransform` (`SceneComponent.K2_GetComponentLocation` (`self.Text3D`))))
  (if (`self.FullyGrown?`)
    (`ActorComponent.K2_DestroyComponent` (`self.CurrentMesh`))
    (switch `string` (`self.WhatCanBeHarvested?`)
      (:`Default`
        _)
      (:`Wheat`
        (`|SpawnActorFromClass` "/Game/Plants/Loose/BP_Loose_Wheat.BP_Loose_Wheat_C" _returnvalue "Undefined" "OverrideRootScale" null "wheatloose" null))
      (:`Corn`
        (`|SpawnActorFromClass` "/Game/Plants/Loose/BP_Loose_Corn.BP_Loose_Corn_C" _returnvalue "Undefined" "OverrideRootScale" null "cornloose" null))
      (:`Pumpkin`
        (`|SpawnActorFromClass` "/Game/Plants/Loose/BP_Loose_Pumpkin.BP_Loose_Pumpkin_C" _returnvalue "Undefined" "OverrideRootScale" null "pumpkinloose" null)))
    (set `self.FullyGrown?` false)
    (set `self.CurrentMesh` null)
    (set `self.WhatCanBeHarvested?` "")
    (set `self.IsSomethingPlanted?` false)))

(fn `InteractWith`
  (params (PlayerCharacter :type "/Game/Blueprints/BP_ThirdPersonCharacter Object Reference"))
  (returns (ObjectiveID :type String))
  (return ""))

(fn `LookAt`
  (returns (Message :type Text))
  (return ""))

(fn `ToGetCrop`
  (params (WhatCrop :type "/Game/Plants/Structures/PlantsEnum Enum" :default "NewEnumerator0"))
  (returns (Amount :type Integer))
  (return 0))

(fn `UserConstructionScript`)